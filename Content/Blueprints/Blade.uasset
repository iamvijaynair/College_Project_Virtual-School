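; Spinning blade hazard that steps back and forth along its forward axis and restarts the current level on contact.
; Each OnProgress event moves a step counter one unit, reversing at zero and MoveTicks.
; Tick spins the blade and eases it toward the counter's offset from its start position with MoveComponentTo.
; Shortly after each step, any actor overlapping the blade triggers the level reload.
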(event EventBeginPlay
  (Variables|Default|SetStartPosition (Variables|/Script/Engine.SceneComponent|GetRelativeLocation (Variables|Default|GetBlade))))

(event EventTick
  (params (DeltaSeconds :type Float%20%28single-precision%29))
  (bind _blade (Variables|Default|GetBlade))
  (Transformation|AddWorldRotation (Variables|Default|GetBlade) (Math|Rotator|MakeRotator 0.0 0.0 (* DeltaSeconds 1.8e+02)) false false)
  (Components|MoveComponentTo _blade (+ (Variables|Default|GetStartPosition) (* (Transformation|GetActorForwardVector) (* (Variables|Default|GetCurrentMoveTicks) 100))) (Transformation|GetWorldRotation _blade) false false 0.1 false))

(event EventOnProgress
  (Utilities|FlowControl|Sequence
    (:then_0
      (if (Variables|Default|GetMovingForward)
        (if (== (Variables|Default|GetCurrentMoveTicks) (Variables|Default|GetMoveTicks))
          (Variables|Default|SetMovingForward false)
          (Variables|Default|SetCurrentMoveTicks (- (Variables|Default|GetCurrentMoveTicks) 1))
          (else
            (Variables|Default|SetCurrentMoveTicks (+ (Variables|Default|GetCurrentMoveTicks) 1))))
        (elif (== (Variables|Default|GetCurrentMoveTicks) 0)
          (Variables|Default|SetMovingForward true)
          (Variables|Default|SetCurrentMoveTicks (+ (Variables|Default|GetCurrentMoveTicks) 1))
          (else
            (Variables|Default|SetCurrentMoveTicks (- (Variables|Default|GetCurrentMoveTicks) 1))))))
    (:then_1
      (Utilities|FlowControl|Delay 0.2)
      (if (> (Utilities|Array|Length (Collision|GetOverlappingActors (Variables|Default|GetBlade) 0 :!class /Script/Engine.PrimitiveComponent)) 0)
        (bind _returnvalue (Game|GetCurrentLevelName true))
        (Game|OpenLevel(byName) (Utilities|String|StringToName _returnvalue))))))

(fn ConstructionScript
  (|CallParentFunction))