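; Player Blueprint that moves in grid steps with WASD and collects a chain of followers.
; Each step requires a clear CheckerBox probe (HasWallAhead returns true when nothing overlaps), shifts TargetPosition, starts a half-second cooldown and calls OnProgress on every Progressor.
; Tick eases the root component toward TargetPosition.
; Overlapping a new Follower appends it to the chain, targeting the previous follower or the player.
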(event Collision|EventActorBeginOverlap
  (params (OtherActor :type Actor%20Object%20Reference))
  (bind _followers (Variables|Default|GetFollowers))
  (bind _followers_2 (Variables|Default|GetFollowers))
  (bind _asfollower (Utilities|Casting|CastToFollower OtherActor))
  (if (not (Utilities|Array|ContainsItem _followers _asfollower))
    (if (> (Utilities|Array|Length _followers) 0)
      (Default|SetTarget _asfollower (Utilities|Array|Get(acopy) _followers_2 (Utilities|Array|LastIndex _followers_2)))
      (else
        (Default|SetTarget _asfollower self)))
    (Utilities|Array|Add (Variables|Default|GetFollowers) _asfollower)))

(event EventTick
  (params (DeltaSeconds :type Float%20%28single-precision%29))
  (Components|MoveComponentTo (Variables|Default|GetDefaultSceneRoot) (Variables|Default|GetTargetPosition) "0, 0, 0" false false 0.1 false))

(event Input|KeyboardEvents|W
  (params (Key :type Key%20Structure :default "None"))
  (:Pressed
    (bind _canmoveahead (CallFunction|HasWallAhead "100.000000,0.000000,50.000000"))
    (if (and _canmoveahead (Variables|Default|GetCanMove))
      (Variables|Default|SetTargetPosition (+ (Variables|Default|GetTargetPosition) "100.000000, 0, 0"))
      (Utilities|FlowControl|Sequence
        (:then_0
          (Variables|Default|SetCanMove false)
          (Utilities|FlowControl|Delay 0.5)
          (Variables|Default|SetCanMove true))
        (:then_1
          (bind _outactors (Actor|GetAllActorsOfClass "/Game/Blueprints/Progressor.Progressor_C"))
          (for _array_element _outactors
            (Default|OnProgress _array_element)))))))

(event Input|KeyboardEvents|S
  (params (Key :type Key%20Structure :default "None"))
  (:Pressed
    (bind _canmoveahead (CallFunction|HasWallAhead "-100.000000,0.000000,50.000000"))
    (if (and _canmoveahead (Variables|Default|GetCanMove))
      (Variables|Default|SetTargetPosition (+ (Variables|Default|GetTargetPosition) "-100.000000, 0, 0"))
      (Utilities|FlowControl|Sequence
        (:then_0
          (Variables|Default|SetCanMove false)
          (Utilities|FlowControl|Delay 0.5)
          (Variables|Default|SetCanMove true))
        (:then_1
          (bind _outactors (Actor|GetAllActorsOfClass "/Game/Blueprints/Progressor.Progressor_C"))
          (for _array_element _outactors
            (Default|OnProgress _array_element)))))))

(event Input|KeyboardEvents|A
  (params (Key :type Key%20Structure :default "None"))
  (:Pressed
    (bind _canmoveahead (CallFunction|HasWallAhead "0.000000,-100.000000,50.000000"))
    (if (and _canmoveahead (Variables|Default|GetCanMove))
      (Variables|Default|SetTargetPosition (+ (Variables|Default|GetTargetPosition) "0.000000,-100.000000, 0"))
      (Utilities|FlowControl|Sequence
        (:then_0
          (Variables|Default|SetCanMove false)
          (Utilities|FlowControl|Delay 0.5)
          (Variables|Default|SetCanMove true))
        (:then_1
          (bind _outactors (Actor|GetAllActorsOfClass "/Game/Blueprints/Progressor.Progressor_C"))
          (for _array_element _outactors
            (Default|OnProgress _array_element)))))))

(event Input|KeyboardEvents|D
  (params (Key :type Key%20Structure :default "None"))
  (:Pressed
    (bind _canmoveahead (CallFunction|HasWallAhead "0.000000,100.000000,50.000000"))
    (if (and _canmoveahead (Variables|Default|GetCanMove))
      (Variables|Default|SetTargetPosition (+ (Variables|Default|GetTargetPosition) "0.000000,100.000000, 0"))
      (Utilities|FlowControl|Sequence
        (:then_0
          (Variables|Default|SetCanMove false)
          (Utilities|FlowControl|Delay 0.5)
          (Variables|Default|SetCanMove true))
        (:then_1
          (bind _outactors (Actor|GetAllActorsOfClass "/Game/Blueprints/Progressor.Progressor_C"))
          (for _array_element _outactors
            (Default|OnProgress _array_element)))))))

(fn ConstructionScript)

(fn HasWallAhead
  (params (PositionCheck :type Vector))
  (bind _checkerbox (Variables|Default|GetCheckerBox))
  (Transformation|SetRelativeLocation _checkerbox PositionCheck false false)
  (return (== (Utilities|Array|Length (Collision|GetOverlappingActors _checkerbox "/Script/Engine.Actor" :!class /Script/Engine.PrimitiveComponent)) 0)))