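; Follower actor that trails a target actor assigned through SetTarget, which also enables movement.
; Each OnProgress event calls the parent, then samples the target's location as the new destination, so the destination updates per progress step rather than every frame.
; Tick drives MoveComponentTo on the root component to ease toward that stored position over a short interval.
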(event EventBeginPlay
  (Variables|Default|SetTargetPosition (Transformation|GetActorLocation)))

(event EventTick
  (params (DeltaSeconds :type Float%20%28single-precision%29))
  (if (Variables|Default|GetCanMove)
    (Components|MoveComponentTo (Variables|Default|GetDefaultSceneRoot) (Variables|Default|GetTargetPosition) "0, 0, 0" false false 0.1 false)))

(event EventOnProgress
  (|CallParentFunction)
  (if (Variables|Default|GetCanMove)
    (Variables|Default|SetTargetPosition (Transformation|GetActorLocation (Variables|Default|GetTarget)))))

(fn ConstructionScript)

(fn SetTarget
  (params (TargetToSet :type Actor%20Object%20Reference))
  (Variables|Default|SetTarget TargetToSet)
  (Variables|Default|SetCanMove true))