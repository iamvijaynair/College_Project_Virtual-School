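; EndGoal is a level exit actor that sends the player on to another level.
; On overlap it casts the actor to Player and checks that its follower count exactly equals FollowersToCollect.
; When they match, it adds a LoadingScreenWidget to the viewport, waits through a fixed delay, then opens the level named by LevelToGoTo.
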(event Collision|EventActorBeginOverlap
  (params (OtherActor :type Actor%20Object%20Reference))
  (bind _asplayer (Utilities|Casting|CastToPlayer OtherActor))
  (if (== (Utilities|Array|Length (Variables|/Game/Blueprints/Player.Player_C|GetFollowers _asplayer)) (Variables|/Game/Blueprints/Player.Player_C|GetFollowersToCollect _asplayer))
    (bind _returnvalue (UserInterface|CreateWidget "/Game/Ui/LoadingScreen/LoadingScreenWidget.LoadingScreenWidget_C"))
    (UserInterface|Viewport|AddtoViewport _returnvalue 0)
    (Utilities|FlowControl|Delay 5.0)
    (Game|OpenLevel(byName) (Variables|Default|GetLevelToGoTo))))

(fn ConstructionScript)